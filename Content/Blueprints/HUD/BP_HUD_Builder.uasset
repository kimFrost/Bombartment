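; BP_HUD_Builder is a HUD Blueprint that draws a dark red line grid across the whole screen.
; On each DrawHUD event it stores the screen size and center, then derives line counts from GridSpacing.
; The horizontal-line loop is nested inside the vertical-line loop, so every horizontal line is redrawn once per vertical line.
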(event `self.ReceiveDrawHUD`
  (params (SizeX :type Integer) (SizeY :type Integer))
  (bind _gridspacing (`self.GridSpacing`))
  (bind _returnvalue (`KismetMathLibrary.MakeVector2D` (`KismetMathLibrary.Conv_IntToDouble` SizeX) (`KismetMathLibrary.Conv_IntToDouble` SizeY)))
  (bind (_x _y) (`KismetMathLibrary.BreakVector2D` (`self.ScreenDimensions`)))
  ;[1 1 1] Set Screen Dimensions
  (set `self.ScreenDimensions` _returnvalue)
  (set `self.ScreenCenterDimensions` (/ _returnvalue 2.0))
  ;[1 1 1] Draw Grid
  (for _index (range (+ (`KismetMathLibrary.FFloor` (/ _x _gridspacing)) 1))
    (bind _returnvalue_2 (* _index (`self.GridSpacing`)))
    (`self.DrawLine` _returnvalue_2 0.0 _returnvalue_2 (`.Y` (`KismetMathLibrary.BreakVector2D` (`self.ScreenDimensions`))) (struct :`R` 0.075926 :`B` 0.016068 :`A` 1.0))
    (for _index_2 (range (+ (`KismetMathLibrary.FFloor` (/ _y _gridspacing)) 1))
      (bind _returnvalue_3 (* _index_2 (`self.GridSpacing`)))
      (`self.DrawLine` 0.0 _returnvalue_3 (`KismetMathLibrary.BreakVector2D` (`self.ScreenDimensions`)) _returnvalue_3 (struct :`R` 0.075926 :`B` 0.016068 :`A` 1.0)))))

(fn `UserConstructionScript`)