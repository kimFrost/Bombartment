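; Main menu HUD that draws New Game and Exit Game buttons on the canvas instead of using widgets.
; DrawHUD centers the menu when ShowMenu is set, adding a bottom-right "Loading" label if ShowLoadingScreen is also set.
; DrawButton renders texture and centered text and registers a hitbox.
; Hitbox release handles opening Minimal_Default or quitting; game-state and loading-flag nodes are disconnected.
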(event `self.ReceiveDrawHUD`
  (params (SizeX :type Integer) (SizeY :type Integer))
  (bind (_outwidth _outheight) (`self.GetTextSize` "Loading" "/Engine/EngineFonts/RobotoDistanceField.RobotoDistanceField"))
  (bind _returnvalue (`KismetMathLibrary.MakeVector2D` (`KismetMathLibrary.Conv_IntToDouble` SizeX) (`KismetMathLibrary.Conv_IntToDouble` SizeY)))
  (bind (_x _y) (`KismetMathLibrary.BreakVector2D` (- (`self.ScreenDimensions`) (`KismetMathLibrary.MakeVector2D` 20.0 20.0))))
  (set `self.GameStateObject` (`GameplayStatics.GetGameState`))
  ;[1 1 1] Set Screen Dimensions
  (set `self.ScreenDimensions` _returnvalue)
  (set `self.ScreenCenterDimensions` (/ _returnvalue 2.0))
  ;[1 1 1] Draw Menu
  (if (`self.ShowMenu`)
    (`self.DrawButton` (- (`self.ScreenCenterDimensions`) (`KismetMathLibrary.MakeVector2D` 0.0 64.0)) "New Game" "NewGame" (select `bool` false :!type "Texture2D Object Reference"))
    (`self.DrawButton` (+ (`self.ScreenCenterDimensions`) (`KismetMathLibrary.MakeVector2D` 0.0 64.0)) "Exit Game" "ExitGame" (select `bool` false :!type "Texture2D Object Reference"))
    ;[1 1 1] Draw Loading Screen
    (if (`self.ShowLoadingScreen`)
      (`self.DrawText` "Loading" (struct :`R` 0.420133 :`G` 0.068875 :`B` 0.725 :`A` 1.0) (- _x _outwidth) (- _y _outheight)))))

(event `self.ReceiveHitBoxClick`
  (params (BoxName :type Name))
  ;[1 1 1] Hit box events
  (switch `name` BoxName))

(event `self.ReceiveHitBoxRelease`
  (params (BoxName :type Name))
  ;[1 1 1] Hit box events
  (switch `name` BoxName
    (:`NewGame`
      (`GameplayStatics.OpenLevel` "Minimal_Default"))
    (:`ExitGame`
      (`KismetSystemLibrary.QuitGame` null))))

(fn `DrawButton`
  (params (`Screen location` :type "Object.Vector2D Structure") (Text :type String) (`Hitbox Name` :type Name) (Texture :type "Texture2D Object Reference"))
  (bind (_outwidth _outheight) (`self.GetTextSize` Text "/Engine/EngineFonts/RobotoDistanceField.RobotoDistanceField" 1.5))
  (bind _returnvalue (- `Screen location` (`KismetMathLibrary.MakeVector2D` 128.0 64.0)))
  (bind (_x _y) (`KismetMathLibrary.BreakVector2D` _returnvalue))
  (bind (_x_2 _y_2) (`KismetMathLibrary.BreakVector2D` (- `Screen location` (/ (`KismetMathLibrary.MakeVector2D` _outwidth _outheight) 2.0))))
  (`self.DrawTextureSimple` Texture _x _y)
  (`self.DrawText` Text (struct :`R` 1.0 :`G` 1.0 :`B` 1.0 :`A` 1.0) _x_2 _y_2 "/Engine/EngineFonts/RobotoDistanceField.RobotoDistanceField" 1.5)
  (`self.AddHitBox` _returnvalue (`KismetMathLibrary.MakeVector2D` 256.0 128.0) `Hitbox Name`))

(fn `UserConstructionScript`)