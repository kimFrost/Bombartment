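; Player controller for an overhead-style camera that moves the controlled pawn along fixed world axes, with pitch clamped every tick.
; Holding right mouse enables pitch look, while yaw turning is left unwired.
; Zoom inputs step the pawn vertically through shared logic.
; Left-click release debug-traces from the MyCharacter camera, multiplying location by scaled forward vector for the endpoint, and prints any hit MyPawn's name.
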(event `self.ReceiveTick`
  (params (DeltaSeconds :type "Float (single-precision)"))
  ;[1 1 1] Restrict Camera Angle
  (`self.SetControlRotation` (`KismetMathLibrary.MakeRot` (`KismetMathLibrary.FClamp` (.pitch (`self.GetControlRotation`)) 290.0 340.0) (.yaw (`self.GetControlRotation`)) (.roll (`self.GetControlRotation`)))))

(event `InputAxis|Forward`
  (params (AxisValue :type "Float (single-precision)"))
  ;[1 1 1] Movement x/y
  (`Pawn.AddMovementInput` (`self.GetControlledPawn`) (`KismetMathLibrary.MakeVector` -1.0 0.0) AxisValue))

(event `InputAxis|Turn`
  (params (AxisValue :type "Float (single-precision)"))
  ;[1 1 1] Turn / Look
)

(event `Key|RightMouseButton`
  ;[1 1 1] Turn / Look
  (:`Pressed`
    (set `self.RightMouseButtonDown` true))
  (:`Released`
    (set `self.RightMouseButtonDown` false)))

(event `InputAxis|Right`
  (params (AxisValue :type "Float (single-precision)"))
  ;[1 1 1] Movement x/y
  (`Pawn.AddMovementInput` (`self.GetControlledPawn`) (`KismetMathLibrary.MakeVector` 0.0 -1.0 -1.0) AxisValue))

(event `InputAxis|LookUp`
  (params (AxisValue :type "Float (single-precision)"))
  ;[1 1 1] Turn / Look
  (if (`self.RightMouseButtonDown`)
    (`self.AddPitchInput` AxisValue)))

(event `Key|LeftMouseButton`
  (:`Released`
    (bind _asmycharacter_c (cast `/Game/Blueprints/Character/MyCharacter` (`self.GetControlledPawn`)))
    (bind _cameracomponent (`/Game/Blueprints/Character/MyCharacter.CameraComponent` _asmycharacter_c))
    (bind _returnvalue (`SceneComponent.K2_GetComponentLocation` _cameracomponent))
    (bind (_outhit _returnvalue_2) (`KismetSystemLibrary.LineTraceSingle` :`Start` _returnvalue :`End` (* _returnvalue (* (`SceneComponent.GetForwardVector` _cameracomponent) 5000.0)) :`TraceChannel` "TraceTypeQuery1" :`DrawDebugType` "Persistent"))
    (if _returnvalue_2
      (bind _asmypawn_c (cast `/Game/Blueprints/Pawn/MyPawn` (`.HitActor` (`GameplayStatics.BreakHitResult` _outhit))))
      (`KismetSystemLibrary.PrintString` (`KismetSystemLibrary.GetDisplayName` _asmypawn_c)))))

(event `InputAction|ZoomIn`
  (bind _returnvalue (`self.GetControlledPawn`))
  ;[1 1 1] Zoom
  (:`Pressed`
    (set `self.ZoomDirection` -1)
    (`self.K2_SetActorLocation` _returnvalue (+ (`self.K2_GetActorLocation` _returnvalue) (`KismetMathLibrary.MakeVector` 0.0 0.0 (`KismetMathLibrary.Conv_IntToDouble` (* (`self.ZomAmount`) (`self.ZoomDirection`))))) false :!label _label)))

(event `InputAction|ZoomOut`
  ;[1 1 1] Zoom
  (:`Pressed`
    (set `self.ZoomDirection` 1)
    (goto _label)))

(fn `UserConstructionScript`)