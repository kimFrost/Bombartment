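; Superseded menu game state Blueprint that persists state flags, such as whether to show the loading screen, through a BP_GameState_SaveGame slot.
; On BeginPlay, InitStates loads the existing slot or creates it, printing the result for debugging.
; Separate LoadStates and SaveStates helpers are never called here, and SaveStates only writes when no slot exists.
; GetState and SetState are stubs, and older save and logging chains are left disconnected.
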(event `self.ReceiveBeginPlay`
  (`self.InitStates`))

(event `ReceiveBeginPlay_Copy`)

(event `GetState_OLD`)

(event `SetState_OLD`)

(fn `GetState`
  (returns (NewParam :type Boolean))
  (return false))

(fn `InitStates`
  (bind _gamestatesavegame (`self.GameStateSaveGame`))
  (bind _gamestatesavegame_2 (`self.GameStateSaveGame`))
  (bind _saveslotname (`/Game/Blueprints/SaveGame/BP_GameState_SaveGame.SaveSlotName` _gamestatesavegame))
  (bind _userindex (`/Game/Blueprints/SaveGame/BP_GameState_SaveGame.UserIndex` _gamestatesavegame))
  (bind _returnvalue (`GameplayStatics.CreateSaveGameObject` "/Game/Blueprints/SaveGame/BP_GameState_SaveGame.BP_GameState_SaveGame_C"))
  (bind _asbp_gamestate_savegame_c (cast `/Game/Blueprints/SaveGame/BP_GameState_SaveGame` _returnvalue)
    (:`then`
      (set `self.GameStateSaveGame` _asbp_gamestate_savegame_c)
      (bind _returnvalue_2 (`GameplayStatics.DoesSaveGameExist` _saveslotname _userindex))
      (if _returnvalue_2
        (bind _returnvalue_3 (`GameplayStatics.LoadGameFromSlot` _saveslotname _userindex))
        (bind _asbp_gamestate_savegame_c_2 (cast `/Game/Blueprints/SaveGame/BP_GameState_SaveGame` _returnvalue_3)
          (:`then`
            (set `self.GameStateSaveGame` _asbp_gamestate_savegame_c_2)
            (`KismetSystemLibrary.PrintString` (`KismetStringLibrary.Conv_BoolToString` (`/Game/Blueprints/SaveGame/BP_GameState_SaveGame.ShowLoadingScreen` (`self.GameStateSaveGame`)))))
          (:`CastFailed`
            (`KismetSystemLibrary.PrintString` "Cast failed")))
        (else
          (bind _returnvalue_4 (`GameplayStatics.SaveGameToSlot` _gamestatesavegame_2 (`/Game/Blueprints/SaveGame/BP_GameState_SaveGame.SaveSlotName` _gamestatesavegame_2) (`/Game/Blueprints/SaveGame/BP_GameState_SaveGame.UserIndex` _gamestatesavegame_2)))
          (`KismetSystemLibrary.PrintString` (`KismetStringLibrary.Concat_StrStr` "Create Save Slot: " (`KismetStringLibrary.Conv_BoolToString` _returnvalue_4))))))
    (:`CastFailed`
      (`KismetSystemLibrary.PrintString` "Cast failed"))))

(fn `LoadStates`
  (bind _gamestatesavegame (`self.GameStateSaveGame`))
  (bind _saveslotname (`/Game/Blueprints/SaveGame/BP_GameState_SaveGame.SaveSlotName` _gamestatesavegame))
  (bind _userindex (`/Game/Blueprints/SaveGame/BP_GameState_SaveGame.UserIndex` _gamestatesavegame))
  (bind _returnvalue (`GameplayStatics.CreateSaveGameObject` "/Game/Blueprints/SaveGame/BP_GameState_SaveGame.BP_GameState_SaveGame_C"))
  (bind _asbp_gamestate_savegame_c (cast `/Game/Blueprints/SaveGame/BP_GameState_SaveGame` _returnvalue)
    (:`then`
      (set `self.GameStateSaveGame` _asbp_gamestate_savegame_c)
      (bind _returnvalue_2 (`GameplayStatics.DoesSaveGameExist` _saveslotname _userindex))
      (if _returnvalue_2
        (bind _returnvalue_3 (`GameplayStatics.LoadGameFromSlot` _saveslotname _userindex))
        (bind _asbp_gamestate_savegame_c_2 (cast `/Game/Blueprints/SaveGame/BP_GameState_SaveGame` _returnvalue_3)
          (:`then`
            (set `self.GameStateSaveGame` _asbp_gamestate_savegame_c_2)
            (`KismetSystemLibrary.PrintString` (`KismetStringLibrary.Conv_BoolToString` (`/Game/Blueprints/SaveGame/BP_GameState_SaveGame.ShowLoadingScreen` (`self.GameStateSaveGame`)))))
          (:`CastFailed`
            (`KismetSystemLibrary.PrintString` "Cast failed")))))
    (:`CastFailed`
      (`KismetSystemLibrary.PrintString` "Cast failed"))))

(fn `SaveStates`
  (bind _gamestatesavegame (`self.GameStateSaveGame`))
  (bind _saveslotname (`/Game/Blueprints/SaveGame/BP_GameState_SaveGame.SaveSlotName` _gamestatesavegame))
  (bind _userindex (`/Game/Blueprints/SaveGame/BP_GameState_SaveGame.UserIndex` _gamestatesavegame))
  (bind _returnvalue (`GameplayStatics.CreateSaveGameObject` "/Game/Blueprints/SaveGame/BP_GameState_SaveGame.BP_GameState_SaveGame_C"))
  (bind _asbp_gamestate_savegame_c (cast `/Game/Blueprints/SaveGame/BP_GameState_SaveGame` _returnvalue)
    (:`then`
      (set `self.GameStateSaveGame` _asbp_gamestate_savegame_c)
      (bind _returnvalue_2 (`GameplayStatics.DoesSaveGameExist` _saveslotname _userindex))
      (if (not _returnvalue_2)
        (bind _returnvalue_3 (`GameplayStatics.SaveGameToSlot` _gamestatesavegame _saveslotname _userindex))
        (`KismetSystemLibrary.PrintString` (`KismetStringLibrary.Concat_StrStr` "Save Save Slot: " (`KismetStringLibrary.Conv_BoolToString` _returnvalue_3)))))
    (:`CastFailed`
      (`KismetSystemLibrary.PrintString` "Cast failed"))))

(fn `SetState`
  (params (variableName :type Name)))

(fn `UserConstructionScript`)