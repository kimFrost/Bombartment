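; Menu game state that owns the BP_GameState_SaveGame object holding the persistent ShowLoadingScreen flag.
; BeginPlay creates the save object, stores the result of its InitSave for the slot, and logs through BP_Menu_HUD.
; GetState only logs the flag to the HUD, while SetState sets it true and calls SaveData.
; Disconnected nodes hold an unused manual slot load/save test with PlayerName.
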(event `self.ReceiveBeginPlay`
  (bind _returnvalue (`GameplayStatics.CreateSaveGameObject` "/Game/Blueprints/SaveGame/BP_GameState_SaveGame.BP_GameState_SaveGame_C"))
  (bind _asbp_gamestate_savegame_c (cast `/Game/Blueprints/SaveGame/BP_GameState_SaveGame` _returnvalue))
  (bind _savegameinstance (`/Game/Blueprints/SaveGame/BP_GameState_SaveGame.InitSave` _asbp_gamestate_savegame_c (`self.SaveSlotName`)))
  (set `self.SaveGame` _savegameinstance)
  (bind _asbp_menu_hud_c (cast `/Game/Blueprints/HUD/BP_Menu_HUD` (`PlayerController.GetHUD` (`GameplayStatics.GetPlayerController` 0))))
  (`/Game/Blueprints/HUD/BP_Menu_HUD.Log` _asbp_menu_hud_c "Init Save" "GameState" true))

(event `GetState`
  (bind _asbp_menu_hud_c (cast `/Game/Blueprints/HUD/BP_Menu_HUD` (`PlayerController.GetHUD` (`GameplayStatics.GetPlayerController` 0)))
    (:`then`
      (`/Game/Blueprints/HUD/BP_Menu_HUD.Log` _asbp_menu_hud_c (`KismetStringLibrary.Concat_StrStr` "ShowLoadingScreen:" (`KismetStringLibrary.Conv_BoolToString` (`/Game/Blueprints/SaveGame/BP_GameState_SaveGame.ShowLoadingScreen` (`self.SaveGame`)))) "GameState" true))
    (:`CastFailed`
      (`KismetSystemLibrary.PrintString` "Cast Fail"))))

(event `SetState`
  (bind _savegame (`self.SaveGame`))
  (set `/Game/Blueprints/SaveGame/BP_GameState_SaveGame.ShowLoadingScreen` true _savegame)
  (`/Game/Blueprints/SaveGame/BP_GameState_SaveGame.SaveData` _savegame))

(fn `UserConstructionScript`)