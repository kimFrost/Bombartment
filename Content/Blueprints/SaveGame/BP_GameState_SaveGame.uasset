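; BP_GameState_SaveGame is a save game Blueprint for game state, with InitSave, SaveData and LoadData functions that are currently empty stubs.
; Their logic is disconnected from the function entries and never runs.
; That unwired logic would load or create a named slot, cache the instance and gate later saves and loads on an Initialized flag, logging through BP_Menu_HUD.
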(fn `InitSave`
  (params (NewParam :type String))
  (returns (SaveGameInstance :type "/Game/Blueprints/SaveGame/BP_GameState_SaveGame Object Reference")))

(fn `LoadData`)

(fn `SaveData`)